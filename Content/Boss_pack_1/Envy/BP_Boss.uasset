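; Envy boss character that shows a health widget, takes damage and hurts the player through limb and tail overlaps gated by combo flags.
; Attack01 plays the combo montage and signals its end; the chase and distance-based attack logic is disconnected, leaving Combo02 and Combo03 never enabled here.
; Non-lethal hits add knockback, blood effects and brief global time-dilation hit-stop.
; Death plays a montage, then destroys the actor and calls a special-effect dispatcher.
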(event OnComponentBeginOverlap(Patinha_Direita)
  (params (OverlappedComponent :type Primitive%20Component%20Object%20Reference) (OtherActor :type Actor%20Object%20Reference) (OtherComp :type Primitive%20Component%20Object%20Reference) (OtherBodyIndex :type Integer) (bFromSweep :type Boolean) (SweepResult :type Hit%20Result%20Structure%20%28by%20ref%29))
  (if (Variables|Default|GetCombo01)
    (bind _asbp_third_person_character (Utilities|Casting|CastToBP_ThirdPersonCharacter OtherActor))
    (Game|Damage|ApplyPointDamage _asbp_third_person_character 2e+01 (Transformation|GetActorLocation))))

(event OnComponentBeginOverlap(Patinha_Esquerda)
  (params (OverlappedComponent :type Primitive%20Component%20Object%20Reference) (OtherActor :type Actor%20Object%20Reference) (OtherComp :type Primitive%20Component%20Object%20Reference) (OtherBodyIndex :type Integer) (bFromSweep :type Boolean) (SweepResult :type Hit%20Result%20Structure%20%28by%20ref%29))
  (if (Variables|Default|GetCombo01)
    (bind _asbp_third_person_character (Utilities|Casting|CastToBP_ThirdPersonCharacter OtherActor))
    (Game|Damage|ApplyPointDamage _asbp_third_person_character 2e+01 (Transformation|GetActorLocation))))

(event OnTargetPerceptionUpdated(AIPerception)
  (params (Actor :type Actor%20Object%20Reference) (Stimulus :type AI%20Stimulus%20Structure)))

(event OnComponentBeginOverlap(MãoDireita)
  (params (OverlappedComponent :type Primitive%20Component%20Object%20Reference) (OtherActor :type Actor%20Object%20Reference) (OtherComp :type Primitive%20Component%20Object%20Reference) (OtherBodyIndex :type Integer) (bFromSweep :type Boolean) (SweepResult :type Hit%20Result%20Structure%20%28by%20ref%29))
  (if (Variables|Default|GetCombo03)
    (bind _asbp_third_person_character (Utilities|Casting|CastToBP_ThirdPersonCharacter OtherActor))
    (Game|Damage|ApplyPointDamage _asbp_third_person_character 2e+01 (Transformation|GetActorLocation))))

(event OnComponentBeginOverlap(Rabo)
  (params (OverlappedComponent :type Primitive%20Component%20Object%20Reference) (OtherActor :type Actor%20Object%20Reference) (OtherComp :type Primitive%20Component%20Object%20Reference) (OtherBodyIndex :type Integer) (bFromSweep :type Boolean) (SweepResult :type Hit%20Result%20Structure%20%28by%20ref%29))
  (if (Variables|Default|GetCombo02)
    (bind _asbp_third_person_character (Utilities|Casting|CastToBP_ThirdPersonCharacter OtherActor))
    (Game|Damage|ApplyPointDamage _asbp_third_person_character 2e+01 (Transformation|GetActorLocation))))

(event Custom|Attack01
  ;[0.15 0.15 0.15 0.5] Combo garra e mão
  (if (not (Variables|Default|GetAttacking?))
    (if (not (Variables|Default|GetDead?))
      (Variables|Default|SetCombo01 true)
      (Variables|Default|SetAttacking? true)
      (Animation|Montage|PlayMontage (Variables|Character|GetMesh) "/Game/Boss_pack_1/Envy/Anim/Anim_Envy_Attack_12_Montage.Anim_Envy_Attack_12_Montage"
        (:OnCompleted
          _)
        (:OnInterrupted
          _))
      (Variables|Default|SetAttacking? false)
      (Variables|Default|SetCombo01 false)
      (Default|CallAttackEnd))))

(event EventBeginPlay
  (UserInterface|CreateWidget "/Game/Boss_pack_1/Envy/WBP_HealthBoss.WBP_HealthBoss_C"))

(event Collision|EventActorBeginOverlap
  (params (OtherActor :type Actor%20Object%20Reference)))

(event Game|Damage|EventAnyDamage
  (params (Damage :type Float%20%28single-precision%29) (DamageType :type Damage%20Type%20Object%20Reference) (InstigatedBy :type Controller%20Object%20Reference) (DamageCauser :type Actor%20Object%20Reference))
  (bind _returnvalue (Game|GetPlayerCharacter 0))
  (bind _returnvalue_2 (Transformation|GetActorLocation))
  (bind _returnvalue_3 (Transformation|GetActorLocation))
  (bind _returnvalue_4 (Transformation|GetActorLocation _returnvalue))
  (bind _returnvalue_5 (- _returnvalue_3 _returnvalue_4))
  (bind _returnvalue_6 (Math|Vector|Normalize _returnvalue_5))
  (bind _returnvalue_7 (* _returnvalue_6 2e+03))
  (Variables|Default|SetHealth (Math|Float|Clamp(Float) (- (Variables|Default|GetHealth) Damage) 0.0 (Variables|Default|GetMaxHealth)))
  (if (or (== (Variables|Default|GetHealth) 0.0) (<= (Variables|Default|GetHealth) 0.0))
    (Variables|Default|SetDead? true)
    (Animation|Montage|PlayMontage (Variables|Character|GetMesh) "/Game/Boss_pack_1/Envy/Anim/Anim_Envy_Death_1_Montage.Anim_Envy_Death_1_Montage" 0.7
      (:OnCompleted
        (Actor|DestroyActor)
        (Default|CallSpawnEfeitoEspecial)))
    (else
      ;[0.15 0.15 0.15 0.5] AnyDamage
      (Physics|AddImpulse (Variables|Character|GetCharacterMovement) (Math|Vector|MakeVector (.x _returnvalue_7) (.y _returnvalue_7) 0.0) true)
      (Utilities|Time|SetGlobalTimeDilation 0.1)
      (Niagara|SpawnSystematLocation "/DismembermentSystem/EnGoreDismembermentSystem/Gore/NS_DIS_BloodBurst.NS_DIS_BloodBurst" _returnvalue_2)
      (Rendering|Decal|SpawnDecalatLocation "/DismembermentSystem/EnGoreDismembermentSystem/Gore/Mats/M_Decal_BloodPool.M_Decal_BloodPool" "100.000000,100.000000,100.000000" _returnvalue_2 "-90.000000,0.000000,0.000000" 0.0)
      (Utilities|FlowControl|Delay 0.009)
      (Utilities|Time|SetGlobalTimeDilation 1.0))))

(event EventTick
  (params (DeltaSeconds :type Float%20%28single-precision%29)))

(fn ConstructionScript)