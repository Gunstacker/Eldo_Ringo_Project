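; Dash_Water is a configurable water actor that exposes surface, caustics and underwater look settings as variables.
; Its construction script creates dynamic materials for the DensePlane water surface and DashCaustics, pushing color, wave, foam, rain and caustic parameters.
; Caustic intensity also scales with water calmness.
; A helper rebuilds the UnderWaterPostProcess settings with bloom and a dynamic blendable material, which then receives fog, blur, warping and brightness values.
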(event EventBeginPlay)

(event Collision|EventActorBeginOverlap
  (params (OtherActor :type Actor%20Object%20Reference)))

(event EventTick
  (params (DeltaSeconds :type Float%20%28single-precision%29)))

(fn ConstructionScript
  (bind _posprocess_material (Variables|Default|GetPosProcess_Material))
  (bind _water_calmness (Variables|Water|GetWater%20Calmness))
  (Utilities|FlowControl|Sequence
    (:then_0
      (bind _returnvalue (Rendering|Material|CreateDynamicMaterialInstance (Variables|Default|GetDensePlane) 0 (Variables|Default|GetSource%20Material) "None" :!class /Script/Engine.PrimitiveComponent))
      ;[0.4037 0.8073 1] Water
      (Rendering|Material|SetScalarParameterValue _returnvalue "Calmness" _water_calmness :!class /Script/Engine.MaterialInstanceDynamic)
      (Rendering|Material|SetVectorParameterValue _returnvalue "Surface_Color" (Variables|Water|GetSurface%20Color) :!class /Script/Engine.MaterialInstanceDynamic)
      (Rendering|Material|SetVectorParameterValue _returnvalue "Depth_Color" (Variables|Water|GetDepth%20Color) :!class /Script/Engine.MaterialInstanceDynamic)
      (Rendering|Material|SetScalarParameterValue _returnvalue "Depth" (Variables|Water|GetWater%20Depth) :!class /Script/Engine.MaterialInstanceDynamic)
      (Rendering|Material|SetScalarParameterValue _returnvalue "Rotation" (Variables|Water|GetRotation) :!class /Script/Engine.MaterialInstanceDynamic)
      (Rendering|Material|SetScalarParameterValue _returnvalue "Foam_Size" (Variables|Water|GetFoam%20Tilling) :!class /Script/Engine.MaterialInstanceDynamic)
      (Rendering|Material|SetScalarParameterValue _returnvalue "Foam_Depth" (Variables|Water|GetFoam%20) :!class /Script/Engine.MaterialInstanceDynamic)
      (Rendering|Material|SetScalarParameterValue _returnvalue "Foam_Proximity" (Variables|Water|GetFoam%20Surface%20Proximity) :!class /Script/Engine.MaterialInstanceDynamic)
      (Rendering|Material|SetScalarParameterValue _returnvalue "Water_Ondulation" (Variables|Water|GetWater%20Ondulation) :!class /Script/Engine.MaterialInstanceDynamic)
      (Rendering|Material|SetScalarParameterValue _returnvalue "Wave_Height" (Variables|Water|GetWave%20Height) :!class /Script/Engine.MaterialInstanceDynamic)
      (Rendering|Material|SetScalarParameterValue _returnvalue "Wave_Ondulation_Strength" (Variables|Water|GetWave%20Ondulation%20Strength) :!class /Script/Engine.MaterialInstanceDynamic)
      (Rendering|Material|SetScalarParameterValue _returnvalue "Wave_Strength" (Variables|Water|GetWave%20Strength) :!class /Script/Engine.MaterialInstanceDynamic)
      (Rendering|Material|SetScalarParameterValue _returnvalue "Wave_Speed" (Variables|Water|GetWave%20Speed) :!class /Script/Engine.MaterialInstanceDynamic)
      (Rendering|Material|SetScalarParameterValue _returnvalue "Wave_Size" (Variables|Water|GetWave%20Size) :!class /Script/Engine.MaterialInstanceDynamic)
      (Rendering|Material|SetScalarParameterValue _returnvalue "Rain" (Variables|Water|GetRain) :!class /Script/Engine.MaterialInstanceDynamic)
      (Rendering|Material|SetScalarParameterValue _returnvalue "T Ripple Size" (Variables|Water|GetRipple%20Tilling) :!class /Script/Engine.MaterialInstanceDynamic))
    (:then_1
      (bind _returnvalue_2 (Rendering|Material|CreateDynamicMaterialInstance (Variables|Default|GetDash_Caustics) :!class /Script/Engine.DecalComponent))
      ;[1 0.3664 0.8557] Caustics
      (Rendering|Material|SetVectorParameterValue _returnvalue_2 "Underlying_Color" (Variables|UnderWaterAndCaustics|GetUnderlying%20Color) :!class /Script/Engine.MaterialInstanceDynamic)
      (Rendering|Material|SetScalarParameterValue _returnvalue_2 "Caustic_Intensity" (* (* _water_calmness 0.6) (Variables|UnderWaterAndCaustics|GetCaustic%20Intensity)) :!class /Script/Engine.MaterialInstanceDynamic)
      (Rendering|Material|SetScalarParameterValue _returnvalue_2 "Caustic_Scale" (Variables|UnderWaterAndCaustics|GetCaustic%20Scale) :!class /Script/Engine.MaterialInstanceDynamic)
      (Rendering|Material|SetScalarParameterValue _returnvalue_2 "Caustics_Speed" (Variables|UnderWaterAndCaustics|GetCaustic%20Speed) :!class /Script/Engine.MaterialInstanceDynamic)
      (Rendering|Material|SetScalarParameterValue _returnvalue_2 "Underlying_Hue" (Variables|UnderWaterAndCaustics|GetUnderlying%20Hue) :!class /Script/Engine.MaterialInstanceDynamic)
      (Rendering|Material|SetScalarParameterValue _returnvalue_2 "Underlying_Saturation" (Variables|UnderWaterAndCaustics|GetUnderlying%20Saturation) :!class /Script/Engine.MaterialInstanceDynamic)
      (Rendering|Material|SetScalarParameterValue _returnvalue_2 "Caustic_Roughness" (Variables|UnderWaterAndCaustics|GetUnderlying%20Roughness) :!class /Script/Engine.MaterialInstanceDynamic)
      (Rendering|Material|SetScalarParameterValue _returnvalue_2 "Rotation" (Variables|UnderWaterAndCaustics|GetCaustic%20Rotation) :!class /Script/Engine.MaterialInstanceDynamic))
    (:then_2
      ;[1 1 1] Under Water Post Process
      (CallFunction|SetPostProcessDynamicMaterial)
      (Rendering|Material|SetScalarParameterValue _posprocess_material "Fog_Distance" (* (Variables|UnderWaterAndCaustics|GetFog%20Distance) 2.0) :!class /Script/Engine.MaterialInstanceDynamic)
      (Rendering|Material|SetScalarParameterValue _posprocess_material "Blurriness" (* (Variables|UnderWaterAndCaustics|GetBlurriness) 0.8) :!class /Script/Engine.MaterialInstanceDynamic)
      (Rendering|Material|SetScalarParameterValue _posprocess_material "UnderWater_Warping " (* (Variables|UnderWaterAndCaustics|GetUnderWater%20Warping%20) 0.02) :!class /Script/Engine.MaterialInstanceDynamic)
      (Rendering|Material|SetScalarParameterValue _posprocess_material "Under_Water_Brightness" (Variables|UnderWaterAndCaustics|GetUnder%20Water%20Brightness) :!class /Script/Engine.MaterialInstanceDynamic)
      (Rendering|Material|SetVectorParameterValue _posprocess_material "UnderWater_Fog_Color" (Variables|UnderWaterAndCaustics|GetUnder%20Water%20Fog%20Color) :!class /Script/Engine.MaterialInstanceDynamic))))

(fn SetPostProcessDynamicMaterial
  ;[1 1 1] Comment
  (bind _returnvalue (Rendering|Material|CreateDynamicMaterialInstance (Variables|Default|GetParent) "None" "None" :!class /Script/Engine.KismetMaterialLibrary))
  (Variables|Default|SetPosProcess_Material _returnvalue)
  (bind _structout (Utilities|Struct|SetmembersinPostProcessSettings (Utilities|Struct|MakePostProcessSettings "(Array=)") (Variables|UnderWaterAndCaustics|GetBloom%20Intensity) (Utilities|Struct|MakeWeightedBlendables (Utilities|Array|MakeArray (Utilities|Struct|MakeWeightedBlendable 1.0 (Variables|Default|GetPosProcess_Material))))))
  (Variables|/Script/Engine.PostProcessComponent|SetSettings (Variables|Default|GetUnderWater_PostProcess) _structout))